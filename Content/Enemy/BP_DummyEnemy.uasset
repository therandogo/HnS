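; BP_DummyEnemy is an enemy test dummy with a health component and a generic AI controller.
; On BeginPlay it initializes the C++ health component with a starting health set above its maximum.
; Any health change calls OnHitWhenUnalert, which calls SetPlayerKey on the AI controller, with no check of alert state.
; Tick prints current health on screen every frame as debug output.
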(event OnHealthChangedSignature(BPC_CPP_Health)
  (params (delta :type Float%20%28single-precision%29))
  (CallFunction|OnHitwhenUnalert))

(event EventTick
  (params (DeltaSeconds :type Float%20%28single-precision%29))
  (Development|PrintString (Utilities|String|ToString(Float) (Class|BPCCPPHealthComponent|GetCurrentHealth (Variables|Default|GetBPC_CPP_Health))) true true "(R=0.000000,G=0.660000,B=1.000000,A=1.000000)" 0.01))

(event EventBeginPlay
  (CallFunction|InitializeHealth))

(fn ConstructionScript)

(fn OnHitwhenUnalert
  (bind _asaic_generic_controller (Utilities|Casting|CastToAIC_GenericController (Pawn|GetController)))
  (Default|SetPlayerKey _asaic_generic_controller))

(fn InitializeHealth
  (Class|BPCCPPHealthComponent|InitializeHealth (Variables|Default|GetBPC_CPP_Health) 1.5e+02 1e+02))