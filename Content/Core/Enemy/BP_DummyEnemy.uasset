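; Dummy enemy character with a health component, a health bar widget and an AI controller.
; Damage plays a hit-react montage that updates the bar, messages the player pawn on notify and tells the controller of the hit on completion.
; Death flags the controller, ragdolls the mesh, disables capsule collision and hides the bar.
; A fast looping timer switches the widget between screen and world space by player distance.
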(event OnDeathSignature(BPC_CPP_Health)
  (params (delta :type Float%20%28single-precision%29))
  (CallFunction|DeathFunction))

(event OnHealthChangedSignature(BPC_CPP_Health)
  (params (delta :type Float%20%28single-precision%29))
  (Animation|Montage|PlayMontage (Variables|Character|GetMesh) "/Game/Characters/Mannequins/Animations/HitReact/HitReact_UE_Montage.HitReact_UE_Montage"
    (:then
      (CallFunction|UIHealthFunction))
    (:OnCompleted
      (CallFunction|OnHit))
    (:OnNotifyBegin
      (Class|BPIonEnemyHit|EnemyHitSuccessfuly(Message) (Game|Player|GetPlayerPawn 0)))))

(event Custom|Cull%20UI
  (bind _uiwidget (Variables|Default|GetUIWidget))
  (if (> (Transformation|GetHorizontalDistanceTo (Game|Player|GetPlayerPawn 0)) 5e+02)
    (Class|WidgetComponent|SetWidgetSpace _uiwidget "World")
    (else
      (Class|WidgetComponent|SetWidgetSpace _uiwidget "Screen"))))

(event EventBeginPlay
  (CallFunction|InitializeHealth)
  (Utilities|Time|SetTimerbyEvent (delegate Custom|Cull%20UI) 0.01 true))

(fn ConstructionScript)

(fn OnHit
  (bind _asaic_generic_controller (Utilities|Casting|CastToAIC_GenericController (Pawn|GetController)))
  (Default|SetPlayerKey _asaic_generic_controller)
  (Default|IsHit _asaic_generic_controller))

(fn InitializeHealth
  (Class|BPCCPPHealthComponent|InitializeHealth (Variables|Default|GetBPC_CPP_Health) 1.5e+02 1e+02))

(fn UIHealthFunction
  (bind _bpc_cpp_health (Variables|Default|GetBPC_CPP_Health))
  (Class|BPIEntitytoUI|UpdateHealthFunction(Message) (UserInterface|GetWidget (Variables|Default|GetUIWidget)) (/ (Class|BPCCPPHealthComponent|GetCurrentHealth _bpc_cpp_health) (Class|BPCCPPHealthComponent|GetMaxHealth _bpc_cpp_health))))

(fn DeathFunction
  (bind _mesh (Variables|Character|GetMesh))
  (bind _asaic_generic_controller (Utilities|Casting|CastToAIC_GenericController (Pawn|GetController)))
  (Default|IsEnemyDummy _asaic_generic_controller true)
  (Collision|SetCollisionProfileName _mesh "Ragdoll" true :!class /Script/Engine.PrimitiveComponent)
  (Physics|SetSimulatePhysics _mesh true)
  (Rendering|SetVisibility (Variables|Default|GetUIWidget) false false)
  (Collision|SetCollisionEnabled (Variables|Collision|GetCapsuleComponent) "NoCollision"))