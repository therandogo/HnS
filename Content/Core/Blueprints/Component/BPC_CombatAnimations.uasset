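; Combat component that plays melee-style combo attack montages on the owning actor's skeletal mesh from input type and actor state.
; SendInput searches ComboList for an attack at the current combo step matching both, requiring follow-ups to pass CanAttack and share the recorded combo history.
; Matches advance the step and play their montage at its play rate; completion resets the combo and notifies the owner via AttackAnimationCompleteMessage.
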(event Custom|ExecuteMontage
  (params (Montage :type Anim%20Montage%20Object%20Reference) (PlayRate :type Float%20%28double-precision%29))
  (bind _skeletalmeshcomponent (Variables|Owner|GetSkeletalMeshComponent)
    (:then
      (Utilities|IsValid Montage
        (:Is%20Valid
          (Animation|Montage|PlayMontage _skeletalmeshcomponent Montage PlayRate
            (:OnCompleted
              _)))
        (:Is%20Not%20Valid
          (Utilities|FlowControl|Delay 0.1)))
      (CallFunction|ResetCombo)
      (Class|BPISetActorState|AttackAnimationComplete(Message) (Variables|Owner|GetOwningActor)))
    (:else)))

(event EventBeginPlay
  (CallFunction|InitializeComponent))

(fn SendInput
  (params (InputType :type E_InputType%20Enum :default "NewEnumerator0") (ActorState :type E_ActorState%20Enum :default "NewEnumerator0"))
  (if (== (Variables|Combo|GetComboNumber) 0)
    (for _array_element (Variables|/Game/Core/Data/DataAssets/PrimaryDataAssets/ComboData/PDA_ComboList.PDA_ComboList_C|GetCombos (Variables|Combo|GetComboList)) :!label _label
      (Utilities|IsValid _array_element
        (:Is%20Valid
          (Variables|Combo|SetAttackDoesntExist false)
          (if (Utilities|Array|IsValidIndex (Variables|/Game/Core/Data/DataAssets/PrimaryDataAssets/ComboData/PDA_Combo.PDA_Combo_C|GetAttacks _array_element) (Variables|Combo|GetComboNumber))
            (Utilities|IsValid (Utilities|Array|Get(acopy) (Variables|/Game/Core/Data/DataAssets/PrimaryDataAssets/ComboData/PDA_Combo.PDA_Combo_C|GetAttacks _array_element) (Variables|Combo|GetComboNumber))
              (:Is%20Valid
                (if (Utilities|Enum|Equal(Enum) InputType (Variables|/Game/Core/Data/DataAssets/PrimaryDataAssets/ComboData/PDA_Attack.PDA_Attack_C|GetInputTypeRequirement (Utilities|Array|Get(acopy) (Variables|/Game/Core/Data/DataAssets/PrimaryDataAssets/ComboData/PDA_Combo.PDA_Combo_C|GetAttacks _array_element) (Variables|Combo|GetComboNumber))))
                  (for _array_element_2 (Variables|/Game/Core/Data/DataAssets/PrimaryDataAssets/ComboData/PDA_Attack.PDA_Attack_C|GetActorStateRequirement (Utilities|Array|Get(acopy) (Variables|/Game/Core/Data/DataAssets/PrimaryDataAssets/ComboData/PDA_Combo.PDA_Combo_C|GetAttacks _array_element) (Variables|Combo|GetComboNumber)))
                    (if (Utilities|Enum|Equal(Enum) ActorState _array_element_2)
                      (if (== (Variables|Combo|GetComboNumber) 0)
                        (Utilities|Array|Add (Variables|Combo|GetComboHistory) (Utilities|Array|Get(acopy) (Variables|/Game/Core/Data/DataAssets/PrimaryDataAssets/ComboData/PDA_Combo.PDA_Combo_C|GetAttacks _array_element) (Variables|Combo|GetComboNumber)) :!label _label_2)
                        (CallFunction|ExecuteMontage (Variables|/Game/Core/Data/DataAssets/PrimaryDataAssets/ComboData/PDA_Attack.PDA_Attack_C|GetAnimation (Utilities|Array|Get(acopy) (Variables|/Game/Core/Data/DataAssets/PrimaryDataAssets/ComboData/PDA_Combo.PDA_Combo_C|GetAttacks _array_element) (Variables|Combo|GetComboNumber))) (Variables|/Game/Core/Data/DataAssets/PrimaryDataAssets/ComboData/PDA_Attack.PDA_Attack_C|GetPlayRate (Utilities|Array|Get(acopy) (Variables|/Game/Core/Data/DataAssets/PrimaryDataAssets/ComboData/PDA_Combo.PDA_Combo_C|GetAttacks _array_element) (Variables|Combo|GetComboNumber))))
                        (Math|Integer|IncrementInt (Variables|Combo|GetComboNumber)
                          (:%20%20
                            (return)))
                        (else
                          (bind _array_element_3 (Utilities|Array|ForEachLoopwithBreak (Variables|Combo|GetComboHistory) :!label _label_3)
                            (:LoopBody
                              (if (not (Utilities|Array|ContainsItem (Variables|/Game/Core/Data/DataAssets/PrimaryDataAssets/ComboData/PDA_Combo.PDA_Combo_C|GetAttacks _array_element) _array_element_3))
                                (Variables|Combo|SetAttackDoesntExist true)
                                (goto _label_3 Break)))
                            (:Completed
                              (if (not (Variables|Combo|GetAttackDoesntExist))
                                (goto _label_2)))))))))))
            (else
              (Development|PrintString "NO"))))))
    (elif (Variables|Combo|GetCanAttack)
      (goto _label))))

(fn InitializeComponent
  (bind _output_get (Variables|Owner|SetOwningActor (Components|GetOwner)))
  (Variables|Owner|SetSkeletalMeshComponent (Actor|GetComponentbyClass _output_get "/Script/Engine.SkeletalMeshComponent")))

(fn ResetCombo
  (Variables|Combo|SetComboNumber 0)
  (Utilities|Array|Clear (Variables|Combo|GetComboHistory)))